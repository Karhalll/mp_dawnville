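; MOD_MapBeacon is a Blueprint that records a flat rectangular area, apparently for map use, from its Plane component.
; On BeginPlay it stores the Plane bounds' XY center in Origin and the X and Y half-extents in ScaleX and ScaleY.
; An unconnected older variant derives the same values from a Box extent and the actor location, and the construction script is empty.
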(event `self.ReceiveBeginPlay`
  (bind (_origin _boxextent) (`KismetSystemLibrary.GetComponentBounds` (`self.Plane`)))
  (set `self.Origin` (`KismetMathLibrary.Conv_VectorToVector2D` _origin))
  (set `self.ScaleX` (.x _boxextent))
  (set `self.ScaleY` (.y _boxextent)))

(fn `UserConstructionScript`)